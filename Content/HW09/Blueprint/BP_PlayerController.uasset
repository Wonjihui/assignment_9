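; Player controller for a chat-driven game that creates the local player's chat input and notification widgets.
; Submitted messages are prefixed with player info from BP_PlayerState, printed locally, and sent by server RPC to BP_GameMode along with the sending controller.
; A client RPC lets incoming messages be printed on screen through MyPrintString.
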(event Custom|ClientRPCPrintChatMessageString
  (params (InChatMessageString :type String))
  (CallFunction|PrintChatMessageString InChatMessageString))

(event Custom|ServerRPCPrintChatMessageString
  (params (InChatMessageString :type String))
  (Utilities|IsValid (Game|GetGameMode)
    (:Is%20Valid
      (bind _asbp_game_mode (Utilities|Casting|CastToBP_GameMode (Game|GetGameMode)))
      (Default|PrintChatMessageString _asbp_game_mode self InChatMessageString))))

(event EventBeginPlay
  (if (Pawn|IsLocalController)
    (bind _returnvalue (UserInterface|CreateWidget "/Game/HW09/UI/WBP_ChatInput.WBP_ChatInput_C" self))
    (bind _output_get (Variables|Default|SetChatInputWidgetInstance _returnvalue))
    (UserInterface|Viewport|AddtoViewport _output_get 0)
    (bind _returnvalue_2 (UserInterface|CreateWidget "/Game/HW09/UI/WBP_NotificationText.WBP_NotificationText_C" self))
    (bind _output_get_2 (Variables|Default|SetNotificationTextWidgetInstance _returnvalue_2))
    (UserInterface|Viewport|AddtoViewport _output_get_2 0)))

(event EventTick
  (params (DeltaSeconds :type Float%20%28single-precision%29)))

(fn ConstructionScript)

(fn SetChatMessageString
  (params (InChatMessageString :type String))
  (Variables|Default|SetChatMessageString InChatMessageString)
  (bind _asbp_player_state (Utilities|Casting|CastToBP_PlayerState (Game|GetPlayerState 0)))
  (if (Pawn|IsLocalController)
    (CallFunction|ServerRPCPrintChatMessageString (Utilities|String|Append (Utilities|String|Append (Default|GetPlayerInfoString _asbp_player_state) ":") (Variables|Default|GetChatMessageString)))
    (CallFunction|PrintChatMessageString (Utilities|String|Append (Utilities|String|Append (Default|GetPlayerInfoString _asbp_player_state) ":") (Variables|Default|GetChatMessageString)))))

(fn PrintChatMessageString
  (params (InChatMessageString :type String))
  (Class|HW09NetBlueprintFunctionLibrary|MyPrintString self InChatMessageString 1e+01 "(B=255,G=255,R=0,A=255)"))