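; Game mode for a multiplayer chat-based number guessing game where three strikes against a secret number wins.
; PostLogin registers each player controller, assigns a numbered name and multicasts the login through the GameState.
; PrintChatMessageString judges chat lines ending in a valid guess and relays messages to all players via client RPCs.
; JudgeGame announces a win, or a draw when all players exhaust their guesses, then calls ResetGame.
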(event EventBeginPlay
  (bind _returnvalue (Class|HW09NetBlueprintFunctionLibrary|GenerateSecretNumber))
  (Variables|Default|SetSecretNumberString _returnvalue))

(event EventPostLogin
  (params (NewPlayer :type Player%20Controller%20Object%20Reference))
  (bind _asbp_player_controller (Utilities|Casting|CastToBP_PlayerController NewPlayer))
  (Variables|/Game/HW09/Blueprint/BP_PlayerController.BP_PlayerController_C|SetNotificationText _asbp_player_controller "Connected to the game server.")
  (Utilities|Array|Add (Variables|Default|GetAllPlayerControllers) _asbp_player_controller)
  (bind _asbp_player_state (Utilities|Casting|CastToBP_PlayerState (Variables|/Script/Engine.Controller|GetPlayerState _asbp_player_controller)))
  (bind _output_get (Variables|/Game/HW09/Blueprint/BP_PlayerState.BP_PlayerState_C|SetPlayerNameState _asbp_player_state (Utilities|String|Append (Utilities|String|MakeLiteralString) (Utilities|String|ToString(Integer) (Utilities|Array|Length (Variables|Default|GetAllPlayerControllers))))))
  (bind _asbp_game_state (Utilities|Casting|CastToBP_GameState (Game|GetGameState)))
  (Default|MulticastRPCBroadcastLoginMessage _asbp_game_state _output_get))

(fn ConstructionScript)

(fn PrintChatMessageString
  (params (InChattingPlayerController :type BP%20Player%20Controller%20Object%20Reference) (InChatMessageString :type String))
  (LocalVariables|SetChattingPlayerController InChattingPlayerController)
  (LocalVariables|SetChatMessageString InChatMessageString)
  (bind _returnvalue (Class|HW09NetBlueprintFunctionLibrary|IsGuessNumberString (Utilities|String|RightChop (LocalVariables|GetChatMessageString) (- (Utilities|String|Len (LocalVariables|GetChatMessageString)) 3))))
  (if _returnvalue
    (bind _returnvalue_2 (Class|HW09NetBlueprintFunctionLibrary|JudgeResult (Variables|Default|GetSecretNumberString) (Utilities|String|RightChop (LocalVariables|GetChatMessageString) (- (Utilities|String|Len (LocalVariables|GetChatMessageString)) 3))))
    (bind _output_get (LocalVariables|SetJudeResultString _returnvalue_2))
    (CallFunction|IncreaseGuessCount (LocalVariables|GetChattingPlayerController))
    (for _array_element (Variables|Default|GetAllPlayerControllers)
      (Default|ClientRPCPrintChatMessageString _array_element (Utilities|String|Append (Utilities|String|Append (LocalVariables|GetChatMessageString) "") (LocalVariables|GetJudeResultString)))
      (CallFunction|JudgeGame (LocalVariables|GetChattingPlayerController) (Math|Conversions|ToInteger(Byte) (Utilities|String|LeftChop _output_get 0))))
    (else
      (for _array_element_2 (Variables|Default|GetAllPlayerControllers)
        (Default|ClientRPCPrintChatMessageString _array_element_2 (LocalVariables|GetChatMessageString))))))

(fn IncreaseGuessCount
  (params (IncreaseGuessCount :type BP%20Player%20Controller%20Object%20Reference))
  (bind _playerstate (Variables|/Script/Engine.Controller|GetPlayerState IncreaseGuessCount))
  (Utilities|IsValid _playerstate
    (:Is%20Valid
      (bind _asbp_player_state (Utilities|Casting|CastToBP_PlayerState _playerstate))
      (Variables|/Game/HW09/Blueprint/BP_PlayerState.BP_PlayerState_C|SetCurrentGuessCount _asbp_player_state (+ (Variables|/Game/HW09/Blueprint/BP_PlayerState.BP_PlayerState_C|GetCurrentGuessCount _asbp_player_state) 0)))))

(fn ResetGame
  (bind _returnvalue (Class|HW09NetBlueprintFunctionLibrary|GenerateSecretNumber))
  (Variables|Default|SetSecretNumberString _returnvalue)
  (for _array_element (Variables|Default|GetAllPlayerControllers)
    (bind _asbp_player_state (Utilities|Casting|CastToBP_PlayerState (Variables|/Script/Engine.Controller|GetPlayerState _array_element)))
    (Variables|/Game/HW09/Blueprint/BP_PlayerState.BP_PlayerState_C|SetCurrentGuessCount _asbp_player_state 0)))

(fn JudgeGame
  (params (IsChattingPlayerController :type BP%20Player%20Controller%20Object%20Reference) (InStrikeCount :type Integer))
  (LocalVariables|SetLoclChattingPalyerController IsChattingPlayerController)
  (if (== InStrikeCount 3)
    (for _array_element (Variables|Default|GetAllPlayerControllers)
      (Utilities|Casting|CastToBP_PlayerState (Variables|/Script/Engine.Controller|GetPlayerState (LocalVariables|GetLoclChattingPalyerController)))
      (Variables|/Game/HW09/Blueprint/BP_PlayerController.BP_PlayerController_C|SetNotificationText _array_element (Utilities|Text|ToText(String) (Utilities|String|Append "" "Is Win!")))
      (CallFunction|ResetGame))
    (else
      (Utilities|FlowControl|Sequence
        (:then_0
          (LocalVariables|SetIsDraw true)
          (for _array_element_2 (Variables|Default|GetAllPlayerControllers)
            (bind _asbp_player_state (Utilities|Casting|CastToBP_PlayerState (Variables|/Script/Engine.Controller|GetPlayerState _array_element_2)))
            (if (< (Variables|/Game/HW09/Blueprint/BP_PlayerState.BP_PlayerState_C|GetCurrentGuessCount _asbp_player_state) (Variables|/Game/HW09/Blueprint/BP_PlayerState.BP_PlayerState_C|GetMaxGuessCount _asbp_player_state))
              (LocalVariables|SetIsDraw false))))
        (:then_1
          (if (LocalVariables|GetIsDraw)
            (for _array_element_3 (Variables|Default|GetAllPlayerControllers)
              (Variables|/Game/HW09/Blueprint/BP_PlayerController.BP_PlayerController_C|SetNotificationText _array_element_3 "Draw...")
              (CallFunction|ResetGame))))))))