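; BP_PlayerState is a Player State Blueprint that holds a player's name and guess count for what appears to be a guessing game.
; GetPlayerInfoString chains Append calls to build a display string from the name, current guess count and maximum, in the form Name[current/max].
; The event graph and construction script hold no logic, and nothing in this file changes the counts.
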(event EventBeginPlay)

(event EventTick
  (params (DeltaSeconds :type Float%20%28single-precision%29)))

(fn ConstructionScript)

(fn GetPlayerInfoString
  (return (Utilities|String|Append (Utilities|String|Append (Utilities|String|Append (Utilities|String|Append (Utilities|String|Append (Variables|Default|GetPlayerNameState) "[") (Utilities|String|ToString(Integer) (Variables|Default|GetCurrentGuessCount))) "/") (Utilities|String|ToString(Integer) (Variables|Default|GetMaxGuessCount))) "]")))